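; Game mode blueprint for a first-person game that runs the start, game-over and game-clear cycle without reloading the level.
; GameStart shows the title UI and cursor, spawns and possesses a character at the player start if needed, freezes its movement and opens doors tagged FirstOpenDoor.
; GameOver and GameClear show timed result widgets, destroy the pawn and its attached actors, clear BP_LevelMission enemies, then call GameStart again.
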(event Custom|GameStart
  (bind _returnvalue (UserInterface|CreateWidget "/Game/UMG/Title/UMG_Title.UMG_Title_C"))
  (bind _output_get (Variables|Default|SetUMG_Title _returnvalue))
  (UserInterface|Viewport|AddtoViewport _output_get 0)
  (Variables|/Script/Engine.PlayerController|SetbShowMouseCursor (Game|GetPlayerController 0) true)
  (bind _asbp_first_person_character_base (Utilities|Casting|CastToBP_FirstPersonCharacterBase (Game|Player|GetPlayerPawn 0) :!label _label)
    (:then
      (Pawn|Components|CharacterMovement|DisableMovement (Variables|/Script/Engine.Character|GetCharacterMovement _asbp_first_person_character_base))
      (bind _outactors (Actor|GetAllActorsOfClasswithTag "/Game/BP/Props/BP_Door.BP_Door_C" "FirstOpenDoor"))
      (for _array_element _outactors
        (Default|Open _array_element)))
    (:CastFailed
      (bind _returnvalue_2 (Game|SpawnActorfromClass "/Game/BP/FirstPersonCharacter/BP_FirstPersonCharacterBase.BP_FirstPersonCharacterBase_C" (Math|Transform|MakeTransform (Transformation|GetActorLocation (Class|GameModeBase|FindPlayerStart (Game|GetPlayerController 0))) "0, 0, 0" "1.000000,1.000000,1.000000") "Undefined" 0 0))
      (Pawn|Possess (Game|GetPlayerController 0) _returnvalue_2)
      (goto _label))))

(event Custom|GameOver
  (bind _returnvalue (Game|Player|GetPlayerPawn 0))
  (bind _returnvalue_2 (UserInterface|CreateWidget "/Game/UMG/Title/UMG_GameOver.UMG_GameOver_C"))
  (UserInterface|Viewport|AddtoViewport _returnvalue_2 0)
  (for _array_element (Actor|GetAttachedActors _returnvalue true false)
    (Actor|DestroyActor _array_element))
  (Actor|DestroyActor _returnvalue)
  (Pawn|UnPossess (Game|GetPlayerController 0))
  (Default|OnDie _returnvalue_2)
  (Utilities|FlowControl|Delay 5.0)
  (Widget|RemovefromParent _returnvalue_2)
  (bind _outactors (Actor|GetAllActorsOfClass "/Game/BP/Mission/BP_LevelMission.BP_LevelMission_C"))
  (for _array_element_2 _outactors
    (Default|ClearEnemies _array_element_2))
  (CallFunction|GameStart))

(event Custom|GameClear
  (bind _returnvalue (Game|Player|GetPlayerPawn 0))
  (bind _returnvalue_2 (UserInterface|CreateWidget "/Game/UMG/Title/UMG_GameClear.UMG_GameClear_C"))
  (UserInterface|Viewport|AddtoViewport _returnvalue_2 0)
  (Default|OnSurvive _returnvalue_2)
  (Utilities|FlowControl|Delay 3.0)
  (Widget|RemovefromParent _returnvalue_2)
  (for _array_element (Actor|GetAttachedActors _returnvalue true false)
    (Actor|DestroyActor _array_element))
  (Actor|DestroyActor _returnvalue)
  (Pawn|UnPossess (Game|GetPlayerController 0))
  (bind _outactors (Actor|GetAllActorsOfClass "/Game/BP/Mission/BP_LevelMission.BP_LevelMission_C"))
  (for _array_element_2 _outactors
    (Default|ClearEnemies _array_element_2))
  (CallFunction|GameStart))

(event EventBeginPlay
  (CallFunction|GameStart))

(event EventTick
  (params (DeltaSeconds :type Float%20%28single-precision%29)))

(fn ConstructionScript)