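; BP_BaseAIController is the base AI controller for enemies, driving them through a behavior tree.
; On BeginPlay it runs its BehaviourTree and sets an initial AI state.
; ChangeAIState writes the given state enum into the AIState blackboard key.
; Stop and start events halt or restart the tree's logic through the BrainComponent.
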(event Custom|ChangeAIState
  (params (State :type E_BaseEnemyState%20Enum :default "NewEnumerator0"))
  (AI|Components|Blackboard|SetValueasEnum (AI|GetBlackboard 0) (Utilities|Name|MakeLiteralName "AIState") State)
  (Development|PrintString "ChangeState"))

(event Custom|StopBehaivourTree
  (AI|Logic|StopLogic (Variables|Default|GetBrainComponent) ""))

(event Custom|StartBehaviourTree
  (AI|Logic|StartLogic (Variables|Default|GetBrainComponent)))

(event EventBeginPlay
  (AI|RunBehaviorTree (Variables|Default|GetBehaviourTree))
  (CallFunction|ChangeAIState "NewEnumerator1"))

(event EventTick
  (params (DeltaSeconds :type Float%20%28single-precision%29)))

(fn ConstructionScript)