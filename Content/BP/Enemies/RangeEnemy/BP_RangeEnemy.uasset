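; BP_RangeEnemy is a ranged enemy that periodically fires a particle-based attack and damages the player.
; A looping timer set on BeginPlay activates the RangeAttack effect every AttackSpan, then deactivates it after a short delay.
; RangeAttack receives the actor as a Niagara-style callback; particle data events print "Hit" and apply ProjectilePower damage to player pawn 0, without checking what was hit.
; The attack sound node is unconnected.
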(event Custom|FireRangeAttack
  (Components|Activation|Activate (Variables|Default|GetRangeAttack) false)
  (Utilities|FlowControl|Delay 1.5)
  (Components|Activation|Deactivate (Variables|Default|GetRangeAttack)))

(event EventBeginPlay
  (|CallParentFunction)
  (Class|NiagaraComponent|SetVariableObject (Variables|Default|GetRangeAttack) "BP_Callback" self)
  (Utilities|Time|SetTimerbyEvent (delegate Custom|FireRangeAttack) (Variables|Default|GetAttackSpan) true))

(event Collision|EventActorBeginOverlap
  (params (OtherActor :type Actor%20Object%20Reference))
  (|CallParentFunction OtherActor) ; This node is disabled and will not be called.\nDrag off pins to build functionality.
)

(event EventTick
  (params (DeltaSeconds :type Float%20%28single-precision%29))
  (|CallParentFunction DeltaSeconds) ; This node is disabled and will not be called.\nDrag off pins to build functionality.
)

(event EventParticleData
  (params (Data :type Array%20of%20Basic%20Particle%20Data%20Structures) (NiagaraSystem :type Niagara%20System%20Object%20Reference) (SimulationPositionOffset :type Vector%20%28by%20ref%29 :default "0, 0, 0"))
  (Development|PrintString "Hit")
  (Game|Damage|ApplyDamage (Game|Player|GetPlayerPawn 0) (Variables|Default|GetProjectilePower) 0 0))

(fn ConstructionScript
  (|CallParentFunction))