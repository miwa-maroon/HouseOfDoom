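; Base enemy Blueprint that damages the player on contact and tracks its own HP.
; Tick yaws it toward the player camera with a -90 offset, billboard-style.
; Capsule hits on the player apply damage, switch BP_BaseAIController's state and restart its behavior tree, then switch state again and re-arm after a delay.
; AnyDamage subtracts HP, but the zero-HP branch and Die event perform no death logic.
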(event OnComponentHit(CapsuleComponent)
  (params (HitComponent :type Primitive%20Component%20Object%20Reference) (OtherActor :type Actor%20Object%20Reference) (OtherComp :type Primitive%20Component%20Object%20Reference) (NormalImpulse :type Vector :default "0, 0, 0") (Hit :type Hit%20Result%20Structure%20%28by%20ref%29))
  (bind _returnvalue (Game|Player|GetPlayerPawn 0))
  (bind _baseaicontroller (Variables|Default|GetBaseAIController))
  (if (== OtherActor _returnvalue)
    (Utilities|FlowControl|DoOnce false :!label _label
      (:Completed
        (Game|Damage|ApplyDamage _returnvalue 1e+01 0 0)
        (Development|PrintString (Utilities|GetDisplayName OtherActor))
        (Default|ChangeAIState _baseaicontroller "NewEnumerator0")
        (Default|StopBehaivourTree _baseaicontroller)
        (Default|StartBehaviourTree (Variables|Default|GetBaseAIController))
        (Utilities|FlowControl|Delay 5.0)
        (Default|ChangeAIState (Variables|Default|GetBaseAIController) "NewEnumerator1")
        (goto _label Reset)))))

(event Custom|Die)

(event EventBeginPlay
  (bind _asbp_base_aicontroller (Utilities|Casting|CastToBP_BaseAIController (AI|GetAIController self)))
  (Variables|Default|SetBaseAIController _asbp_base_aicontroller))

(event Collision|EventActorBeginOverlap
  (params (OtherActor :type Actor%20Object%20Reference)))

(event EventTick
  (params (DeltaSeconds :type Float%20%28single-precision%29))
  (Transformation|SetActorRotation (Math|Rotator|MakeRotator 0.0 0.0 (+ (.yaw (Math|Rotator|FindLookatRotation (Transformation|GetActorLocation) (Camera|GetCameraLocation (Game|GetPlayerCameraManager 0)))) -9e+01))))

(event Game|Damage|EventAnyDamage
  (params (Damage :type Float%20%28single-precision%29) (DamageType :type Damage%20Type%20Object%20Reference) (InstigatedBy :type Controller%20Object%20Reference) (DamageCauser :type Actor%20Object%20Reference))
  (bind _output_get (Variables|Default|SetHP (- (Variables|Default|GetHP) Damage)))
  (Development|PrintString (Utilities|String|ToString(Float) _output_get))
  (if (<= _output_get 0.0)
    (Utilities|FlowControl|DoOnce false)))

(fn ConstructionScript)