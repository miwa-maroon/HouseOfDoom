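; Base weapon Blueprint that can be picked up and fired by a first-person character, configured from a WeaponData asset.
; The construction script applies the data's mesh, fire sound, muzzle offset, muzzle flash and optional projectile class to its components.
; On pickup it destroys the character's current weapon, registers itself and attaches via the TP weapon component.
; Firing briefly activates the Niagara muzzle flash.
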(event OnPickUp(TP_PickUp)
  (params (PickUpCharacter :type House%20Of%20Doom%20Character%20Object%20Reference))
  (bind _asbp_first_person_character_base (Utilities|Casting|CastToBP_FirstPersonCharacterBase PickUpCharacter))
  (bind _currentweapon (Variables|/Game/BP/FirstPersonCharacter/BP_FirstPersonCharacterBase.BP_FirstPersonCharacterBase_C|GetCurrentWeapon _asbp_first_person_character_base)
    (:then
      (Actor|DestroyActor _currentweapon))
    (:else
      _))
  (Variables|/Game/BP/FirstPersonCharacter/BP_FirstPersonCharacterBase.BP_FirstPersonCharacterBase_C|SetCurrentWeapon _asbp_first_person_character_base self)
  (Class|TPWeaponComponent|AttachWeapon (Variables|Default|GetTP_Weapon) _asbp_first_person_character_base))

(event OnFire(TP_Weapon)
  (Components|Activation|Activate (Variables|Default|GetNS_Flush) false)
  (Utilities|FlowControl|Delay 0.1)
  (Components|Activation|Deactivate (Variables|Default|GetNS_Flush)))

(event EventBeginPlay)

(fn ConstructionScript
  (bind _tp_weapon (Variables|Default|GetTP_Weapon))
  (Class|SkinnedMeshComponent|SetSkeletalMesh (Variables|Default|GetSKWeapon) (Variables|/Game/Data/Weapon/P_Data_Weapons.P_Data_Weapons_C|GetWeaponMesh (Variables|Default|GetWeaponData)) true)
  (Variables|/Script/HouseOfDoom.TP_WeaponComponent|SetFireSound (Variables|Default|GetTP_Weapon) (Variables|/Game/Data/Weapon/P_Data_Weapons.P_Data_Weapons_C|GetFireSFX (Variables|Default|GetWeaponData)))
  (Variables|/Script/HouseOfDoom.TP_WeaponComponent|SetMuzzleOffset (Variables|Default|GetTP_Weapon) (Variables|/Game/Data/Weapon/P_Data_Weapons.P_Data_Weapons_C|GetMuzzleLocation (Variables|Default|GetWeaponData)))
  (Class|NiagaraComponent|SetAsset (Variables|Default|GetNS_Flush) (Variables|/Game/Data/Weapon/P_Data_Weapons.P_Data_Weapons_C|GetMuzzleFlash (Variables|Default|GetWeaponData)) true)
  (if (Variables|/Game/Data/Weapon/P_Data_Weapons.P_Data_Weapons_C|GetUsersProjectile (Variables|Default|GetWeaponData))
    (Variables|/Script/HouseOfDoom.TP_WeaponComponent|SetProjectileClass _tp_weapon (Utilities|GetClass (Variables|/Game/Data/Weapon/P_Data_Weapons.P_Data_Weapons_C|GetProjectileReference (Variables|Default|GetWeaponData))))
    (else
      (Variables|/Script/HouseOfDoom.TP_WeaponComponent|SetProjectileClass _tp_weapon 0))))