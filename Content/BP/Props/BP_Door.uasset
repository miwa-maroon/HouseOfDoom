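; BP_Door is a double door prop that swings its two leaves open and shut.
; Open plays the DoorAnimation timeline, which lerps LDoor and RDoor through opposite 90-degree turns in fixed world rotation.
; Close reverses that timeline and fires on any CloseTrigger overlap, while nothing in this Blueprint calls Open.
; The Scary_Door sound plays on every timeline update, in both directions, rather than once per movement.
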(event OnComponentBeginOverlap(CloseTrigger)
  (params (OverlappedComponent :type Primitive%20Component%20Object%20Reference) (OtherActor :type Actor%20Object%20Reference) (OtherComp :type Primitive%20Component%20Object%20Reference) (OtherBodyIndex :type Integer) (bFromSweep :type Boolean) (SweepResult :type Hit%20Result%20Structure%20%28by%20ref%29))
  (CallFunction|Close))

(event Custom|Close
  (bind _doortimeline (Timeline|DoorAnimation Reverse)
    (:Update
      (Transformation|SetWorldRotation (Variables|Default|GetL_Door) (Math|Rotator|Lerp(Rotator) "0, 0, 0" "0,-90.000000, 0" _doortimeline) false false)
      (Transformation|SetWorldRotation (Variables|Default|GetR_Door) (Math|Rotator|Lerp(Rotator) "0,180.000000, 0" "0,270.000000, 0" _doortimeline) false false)
      (Audio|PlaySoundatLocation "/Game/Sound/Door/Scary_Door.Scary_Door" (Transformation|GetActorLocation) "0, 0, 0" 1.0 1.0 0.0 0 0 0 0))))

(event Custom|Open
  (bind _doortimeline (Timeline|DoorAnimation Play)
    (:Update
      (Transformation|SetWorldRotation (Variables|Default|GetL_Door) (Math|Rotator|Lerp(Rotator) "0, 0, 0" "0,-90.000000, 0" _doortimeline) false false)
      (Transformation|SetWorldRotation (Variables|Default|GetR_Door) (Math|Rotator|Lerp(Rotator) "0,180.000000, 0" "0,270.000000, 0" _doortimeline) false false)
      (Audio|PlaySoundatLocation "/Game/Sound/Door/Scary_Door.Scary_Door" (Transformation|GetActorLocation) "0, 0, 0" 1.0 1.0 0.0 0 0 0 0))))

(event EventBeginPlay)

(event Collision|EventActorBeginOverlap
  (params (OtherActor :type Actor%20Object%20Reference)))

(event EventTick
  (params (DeltaSeconds :type Float%20%28single-precision%29)))

(fn ConstructionScript)